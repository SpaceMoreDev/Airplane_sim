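; BP_SplineActor moves an array of actors back and forth along its spline, evenly offset from one another.
; A Timeline, its rate set by TimelineLength, flip-flops direction on finish and drives MoveOnSpline, which wraps distances past the spline's end and sweeps each move.
; The construction script pre-places the actors along the spline.
; Its sphere claims overlapping BP_SplineFollowingActors, removing them from every BP_SplineActor before appending them, allowing handoff between splines.
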(event OnComponentBeginOverlap(Sphere)
  (params (OverlappedComponent :type Primitive%20Component%20Object%20Reference) (OtherActor :type Actor%20Object%20Reference) (OtherComp :type Primitive%20Component%20Object%20Reference) (OtherBodyIndex :type Integer) (bFromSweep :type Boolean) (SweepResult :type Hit%20Result%20Structure%20%28by%20ref%29))
  (bind _asbp_spline_following_actor (Utilities|Casting|CastToBP_SplineFollowingActor OtherActor))
  (CallFunction|ClearActors _asbp_spline_following_actor)
  (Utilities|Array|Add (Variables|Default|GetActors) _asbp_spline_following_actor))

(event Custom|Play%20Timeline
  (params (Reverse :type Boolean))
  (if Reverse
    (bind _alpha (Timeline|Timeline Reverse)
      (:Update
        (CallFunction|MoveonSpline _alpha))
      (:Finished
        (Utilities|FlowControl|FlipFlop
          (:A
            (CallFunction|PlayTimeline true))
          (:B
            (CallFunction|PlayTimeline false)))))
    (else
      (Timeline|Timeline PlayFromStart))))

(event Custom|clearActors
  (params (NewParam :type Actor%20Object%20Reference))
  (bind _outactors (Actor|GetAllActorsOfClass "BP_SplineActor_C"))
  (for _array_element _outactors
    (Utilities|Array|RemoveItem (Variables|BP_SplineActor_C|GetActors _array_element) NewParam)))

(event EventBeginPlay
  (Components|Timeline|SetPlayRate (Variables|Default|GetTimeline) (/ 1.0 (Variables|Default|GetTimelineLength)))
  (CallFunction|PlayTimeline false))

(fn ConstructionScript
  (bind _splinecomponent (Variables|Default|GetSplineComponent))
  (for (_array_element _array_index) (Variables|Default|GetActors)
    (Transformation|SetActorLocationAndRotation _array_element (Spline|GetLocationatDistanceAlongSpline _splinecomponent (* (Variables|Default|GetOffset%20between%20actors) _array_index) "Local") (Spline|GetRotationatDistanceAlongSpline _splinecomponent (* (Variables|Default|GetOffset%20between%20actors) _array_index) "Local"))))

(fn MoveonSpline
  (params (Alpha :type Float%20%28double-precision%29))
  (bind _splinecomponent (Variables|Default|GetSplineComponent))
  (bind _splinecomponent_2 (Variables|Default|GetSplineComponent))
  (bind _returnvalue (Spline|GetSplineLength _splinecomponent))
  (for (_array_element _array_index) (Variables|Default|GetActors)
    (Utilities|IsValid _array_element
      (:Is%20Valid
        (bind _output_get (Variables|Default|SetDistance%20Along%20Spline (+ (Math|Float|Lerp 0.0 (Spline|GetSplineLength (Variables|Default|GetSplineComponent)) Alpha) (* _array_index (Variables|Default|GetOffset%20between%20actors)))))
        (if (> _output_get _returnvalue)
          (Variables|Default|SetDistance%20Along%20Spline (- (Variables|Default|GetDistance%20Along%20Spline) _returnvalue)))
        (Transformation|SetActorLocationAndRotation _array_element (Spline|GetLocationatDistanceAlongSpline _splinecomponent_2 (Variables|Default|GetDistance%20Along%20Spline) "World") (Spline|GetRotationatDistanceAlongSpline _splinecomponent_2 (Variables|Default|GetDistance%20Along%20Spline) "World") true)))))